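; Game mode for a timed sky race through checkpoints, with a countdown before the race timer starts.
; On BeginPlay it binds every BP_Checkpoint to either the lap-finish event or a time-bonus event that restarts the timer with added seconds.
; Finishing clears the timer; both finish and timeout call Game End with Win true, showing WB_WinScreen.
; Win/lose message and BP_WyrmPawn freeze logic are disconnected.
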(event `self.ReceiveBeginPlay`
  (`|ExecutionSequence`
    (:`then_0`
      (bind _outactors (`GameplayStatics.GetAllActorsOfClass` "/Game/Race_Mec/BP_Checkpoint.BP_Checkpoint_C"))
      (for _array_element _outactors
        (if (`/Game/Race_Mec/BP_Checkpoint.IsLapFInished` _array_element)
          (add `/Game/Race_Mec/BP_Checkpoint.Checkpointcross` _array_element (`|CreateDelegate` :!event `Win_Finished`))
          (else
            (add `/Game/Race_Mec/BP_Checkpoint.CheckPointTime` _array_element (`|CreateDelegate` :!event `CheckpointCross`))))))
    (:`then_1`
      (`self.Start_Countdown`))))

(event `Start_Countdown`
  (`KismetSystemLibrary.PrintString` "Hello")
  (`KismetSystemLibrary.Delay` (`self.Coutdown_Duration`))
  (`self.Game_Start`))

(event `PreGame`
  (`KismetSystemLibrary.PrintString` "Get Ready"))

(event `Game_Start`
  (`KismetSystemLibrary.PrintString` "Hello")
  (bind _returnvalue (`KismetSystemLibrary.K2_SetTimerDelegate` (delegate `Out_of_Time`) (`self.Timer_Duration`)))
  (set `self.Time_Remaining` _returnvalue))

(event `Out_of_Time`
  (`self.Game_End` true))

(event `Game_End`
  (params (Win :type Boolean))
  (bind _returnvalue (`|CreateWidget` "/Game/UI/WB_WinScreen.WB_WinScreen_C"))
  (`UserWidget.AddToViewport` _returnvalue 0))

(event `Win_Finished`
  (`KismetSystemLibrary.K2_ClearAndInvalidateTimerHandle` (`self.Time_Remaining`))
  (`self.Game_End` true))

(event `CheckpointCross`
  (params (GivenTime :type Integer))
  (`self.AddTimeToTimer` GivenTime))

(fn `AddTimeToTimer`
  (params (TimeToAdd :type Integer))
  (bind _returnvalue (`KismetSystemLibrary.K2_SetTimerDelegate` (`|CreateDelegate` :!event `Out_of_Time`) (+ (`KismetSystemLibrary.K2_GetTimerRemainingTimeHandle` (`self.Time_Remaining`)) (`local.TimeToAdd`))))
  (set `self.Time_Remaining` _returnvalue))

(fn `UserConstructionScript`)