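; Player-controlled wyrm pawn with physics-based flight, which adds its input mapping and minimap widget on BeginPlay.
; Front and back wing flaps each push the body upward and briefly fire a thruster, damping spin on release or timeout.
; Five or more consecutive flaps of one pair also fire a pitch thruster.
; Roll input rotates the body directly, while stabilize eases pitch, roll and spin toward zero and brake bleeds off velocity.
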(event `self.ReceiveBeginPlay`
  (bind _asplayer_controller (cast `PlayerController` (`self.GetController`)))
  (bind _returnvalue (pcsubsystem `EnhancedInputLocalPlayerSubsystem` _asplayer_controller))
  (`/Engine/EditorBlueprintResources/StandardMacros.IsValid` _returnvalue
    (:`Is Valid`
      (`EnhancedInputSubsystemInterface.AddMappingContext` _returnvalue "/Game/SkyRacePrototype/IMC_WyrmMapping.IMC_WyrmMapping" 0 (struct))
      (bind _returnvalue_2 (`|CreateWidget` "/Game/UI/HUD/WB_MINIMAP.WB_MINIMAP_C" (`GameplayStatics.GetPlayerController` 0)))
      (`UserWidget.AddToViewport` _returnvalue_2 0)
      (set `self.thrusterActiveLength` 0.5)
      (set `self.consistentUpwardFlapForce` (0.0 0.0 4500000.0))
      (set `self.consecutiveFrontFlaps` 0)
      (set `self.consecutiveBackFlaps` 0))))

(event `EnhancedInput|/Game/SkyRacePrototype/IA_FlapFrontWings`
  (params (ActionValue :type Boolean) (ElapsedSeconds :type "Float (double-precision)") (TriggeredSeconds :type "Float (double-precision)") (InputAction :type "InputAction Object Reference" :default "/Game/SkyRacePrototype/IA_FlapFrontWings.IA_FlapFrontWings"))
  (bind _flightbody (`self.FlightBody`))
  (:`Started`
    (set `self.consecutiveBackFlaps` 0)
    (bind _result (`/Engine/EditorBlueprintResources/StandardMacros.IncrementInt` (`self.consecutiveFrontFlaps`))
      (:`  `
        (if (>= _result 5)
          (`ActorComponent.Activate` (`self.IncreasePitchThruster`) false))
        (`PrimitiveComponent.AddForce` (`self.FlightBody`) (`self.consistentUpwardFlapForce`) "None" false)
        (`ActorComponent.Activate` (`self.FrontWingsThruster`) false)
        (`SceneComponent.K2_SetRelativeRotation` (`self.FrontWings`) (struct :`Pitch` -10.0) false false)
        (`KismetSystemLibrary.Delay` (`self.thrusterActiveLength`))
        (`ActorComponent.Deactivate` (`self.FrontWingsThruster`) :!label _label)
        (`ActorComponent.Deactivate` (`self.IncreasePitchThruster`))
        (`PrimitiveComponent.SetPhysicsAngularVelocityInDegrees` _flightbody (* (`PrimitiveComponent.GetPhysicsAngularVelocityInDegrees` _flightbody "None") (0.666 0.666 0.666)) false "None")
        (`SceneComponent.K2_SetRelativeRotation` :`self` (`self.FrontWings`)))))
  (:`Completed`
    (goto _label)))

(event `EnhancedInput|/Game/SkyRacePrototype/IA_FlapBackWings`
  (params (ActionValue :type Boolean) (ElapsedSeconds :type "Float (double-precision)") (TriggeredSeconds :type "Float (double-precision)") (InputAction :type "InputAction Object Reference" :default "/Game/SkyRacePrototype/IA_FlapBackWings.IA_FlapBackWings"))
  (bind _flightbody (`self.FlightBody`))
  (:`Started`
    (set `self.consecutiveFrontFlaps` 0)
    (bind _result (`/Engine/EditorBlueprintResources/StandardMacros.IncrementInt` (`self.consecutiveBackFlaps`))
      (:`  `
        (if (>= _result 5)
          (`ActorComponent.Activate` (`self.DecreasePitchThruster`) false))
        (`PrimitiveComponent.AddForce` (`self.FlightBody`) (`self.consistentUpwardFlapForce`) "None" false)
        (`ActorComponent.Activate` (`self.BackWingsThruster`) false)
        (`SceneComponent.K2_SetRelativeRotation` (`self.BackWings`) (struct :`Pitch` -10.0) false false)
        (`KismetSystemLibrary.Delay` (`self.thrusterActiveLength`))
        (`ActorComponent.Deactivate` (`self.BackWingsThruster`) :!label _label_2)
        (`ActorComponent.Deactivate` (`self.DecreasePitchThruster`))
        (`PrimitiveComponent.SetPhysicsAngularVelocityInDegrees` _flightbody (* (`PrimitiveComponent.GetPhysicsAngularVelocityInDegrees` _flightbody "None") (0.666 0.666 0.666)) false "None")
        (`SceneComponent.K2_SetRelativeRotation` :`self` (`self.BackWings`)))))
  (:`Completed`
    (goto _label_2)))

(event `EnhancedInput|/Game/SkyRacePrototype/IA_Roll`
  (params (ActionValue :type Boolean) (ElapsedSeconds :type "Float (double-precision)") (TriggeredSeconds :type "Float (double-precision)") (InputAction :type "InputAction Object Reference" :default "/Game/SkyRacePrototype/IA_Roll.IA_Roll"))
  (bind _returnvalue (`self.GetInputAxisKeyValue`))
  (:`Triggered`
    (`SceneComponent.K2_AddRelativeRotation` (`self.FlightBody`) (`KismetMathLibrary.MakeRotator` (* _returnvalue 1.0) (* (`self.GetInputAxisKeyValue`) 0.5) (* _returnvalue 1.0)) false false)))

(event `EnhancedInput|/Game/SkyRacePrototype/IA_Stabilize`
  (params (ActionValue :type Boolean) (ElapsedSeconds :type "Float (double-precision)") (TriggeredSeconds :type "Float (double-precision)") (InputAction :type "InputAction Object Reference" :default "/Game/SkyRacePrototype/IA_Stabilize.IA_Stabilize"))
  (bind _flightbody (`self.FlightBody`))
  (bind _flightbody_2 (`self.FlightBody`))
  (:`Triggered`
    (`SceneComponent.K2_SetWorldRotation` _flightbody_2 (`KismetMathLibrary.MakeRotator` (/ (.roll (`SceneComponent.K2_GetComponentRotation` _flightbody_2)) 1.05) (/ (.pitch (`SceneComponent.K2_GetComponentRotation` _flightbody_2)) 1.05) (.yaw (`SceneComponent.K2_GetComponentRotation` _flightbody_2))) false false)
    (`PrimitiveComponent.SetPhysicsAngularVelocityInDegrees` _flightbody (* (`PrimitiveComponent.GetPhysicsAngularVelocityInDegrees` _flightbody "None") (0.95 0.95 0.95)) false "None")))

(event `EnhancedInput|/Game/SkyRacePrototype/IA_Brake`
  (params (ActionValue :type Boolean) (ElapsedSeconds :type "Float (double-precision)") (TriggeredSeconds :type "Float (double-precision)") (InputAction :type "InputAction Object Reference" :default "/Game/SkyRacePrototype/IA_Brake.IA_Brake"))
  (bind _flightbody (`self.FlightBody`))
  (:`Triggered`
    (bind _returnvalue (`PrimitiveComponent.GetPhysicsLinearVelocity` _flightbody "None"))
    (`PrimitiveComponent.SetPhysicsLinearVelocity` _flightbody (* _returnvalue (0.98 0.98 0.95)) false "None")))

(fn `UserConstructionScript`)