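; BP_AmbiencePlayer is an actor that plays an ambient sound while other actors overlap it.
; On BeginPlay it spawns SoundFile attached to its Scene component at half volume, without auto-destroy, and pauses it immediately.
; Begin and end overlap events unpause and pause that stored audio component, with no check on which actor overlaps.
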(event `self.ReceiveBeginPlay`
  (bind _scene (`self.Scene`))
  (bind _returnvalue (`GameplayStatics.SpawnSoundAttached` (`self.soundFile`) _scene "None" (`SceneComponent.K2_GetComponentLocation` _scene) (struct) "KeepRelativeOffset" true 0.5 1.0 0.0 null null false))
  (bind _output_get (set `self.mySound` _returnvalue))
  (`AudioComponent.SetPaused` _output_get true))

(event `self.ReceiveActorBeginOverlap`
  (params (OtherActor :type "Actor Object Reference"))
  (`AudioComponent.SetPaused` (`self.mySound`) false))

(event `self.ReceiveActorEndOverlap`
  (params (OtherActor :type "Actor Object Reference"))
  (`AudioComponent.SetPaused` (`self.mySound`) true))

(fn `UserConstructionScript`)