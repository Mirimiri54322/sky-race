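; BP_WindWall is a wind hazard volume that switches on a radial wind force while a BP_WyrmPawn overlaps it.
; On BeginPlay it sizes the RadialWindForce1 radius from the larger Y or Z world scale of its Cube and turns off auto-activation.
; Actor overlap begin and end events activate and deactivate the force, ignoring other actor types.
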(event `self.ReceiveBeginPlay`
  (bind (_x _y _z) (`KismetMathLibrary.BreakVector3f` (`SceneComponent.K2_GetComponentScale` (`self.Cube`))))
  (set `RadialForceComponent.Radius` (* (* (`KismetMathLibrary.FMax` _y _z) 0.25) 100.0) (`self.RadialWindForce1`))
  (`ActorComponent.SetAutoActivate` (`self.RadialWindForce1`) false))

(event `self.ReceiveActorBeginOverlap`
  (params (OtherActor :type "Actor Object Reference"))
  (cast `/Game/SkyRacePrototype/BP_WyrmPawn` OtherActor)
  (`ActorComponent.Activate` (`self.RadialWindForce1`) false))

(event `self.ReceiveActorEndOverlap`
  (params (OtherActor :type "Actor Object Reference"))
  (cast `/Game/SkyRacePrototype/BP_WyrmPawn` OtherActor)
  (`ActorComponent.Deactivate` (`self.RadialWindForce1`)))

(fn `UserConstructionScript`)